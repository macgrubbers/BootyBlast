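; BP_EnemyTest is a test enemy character that reacts to seeing BP_GoblinWoman and can be defeated through damage.
; PawnSensing sets hasSeenPlayer on the AI controller's Blackboard, which is never cleared here.
; Damage reduces Health, initialized in the construction script; at zero or below it sets isDefeated on the Blackboard and calls Ragdoll.
; Ragdoll simulates physics from the pelvis down the bone chain, adding an impulse from the last requested movement velocity.
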(event `self.ReceiveBeginPlay`)

(event `self.PawnSensing.OnSeePawn`
  (params (Pawn :type "Pawn Object Reference"))
  ; On see pawn
  (cast `/Game/GOBLINA/GoblinTest/BP_GoblinWoman` Pawn)
  (if (not (`self.isDefeated`))
    ;; Consolidate hasSeenPlayer later - they are separate for the Blackboard and Character blueprints
    (bind _output_get (set `self.hasSeenPlayer` true))
    ;; Once set, enemy will always track player - fix later
    (`BlackboardComponent.SetValueAsBool` (`AIBlueprintHelperLibrary.GetBlackboard` (`AIBlueprintHelperLibrary.GetAIController` self)) "hasSeenPlayer" _output_get)))

(event `self.ReceiveAnyDamage`
  (params (Damage :type "Float (single-precision)") (DamageType :type "DamageType Object Reference") (InstigatedBy :type "Controller Object Reference") (DamageCauser :type "Actor Object Reference"))
  ; taking damage
  (bind _output_get (set `self.health` (- (`self.health`) Damage)))
  (if (>= 0.0 _output_get)
    (`BlackboardComponent.SetValueAsBool` (`AIBlueprintHelperLibrary.GetBlackboard` (`AIBlueprintHelperLibrary.GetAIController` self)) "isDefeated" true)
    (`self.Ragdoll`)))

(fn `Ragdoll`
  (locals (NewLocalVar :type "Vector Structure" :default (0.0 0.0 0.0)))
  (bind _mesh (`self.Mesh`))
  (bind _pelvis (`self.pelvis`))
  (`PrimitiveComponent.SetCollisionProfileName` _mesh "Ragdoll" true)
  (`SkeletalMeshComponent.SetAllBodiesBelowSimulatePhysics` _mesh _pelvis true true)
  (`SkeletalMeshComponent.AddImpulseToAllBodiesBelow` (`self.Mesh`) (`CharacterMovementComponent.GetLastUpdateRequestedVelocity` (`self.CharacterMovement`)) _pelvis false true))

(fn `UserConstructionScript`
  (set `self.health` 100.0))