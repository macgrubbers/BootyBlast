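; BP_StupidEnemyTest is a test enemy character with basic sight detection, health and a defeat state.
; PawnSensing prints a debug message when it spots BP_GoblinWoman.
; Damage reduces the health set in the Construction Script, and at zero sets the AI blackboard's isDefeated flag.
; A Ragdoll function, not called here, simulates physics from the pelvis down and applies the last requested movement velocity as an impulse.
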(event `self.ReceiveBeginPlay`)

(event `self.PawnSensing.OnSeePawn`
  (params (Pawn :type "Pawn Object Reference"))
  ; On see pawn
  (cast `/Game/GOBLINA/GoblinTest/BP_GoblinWoman` Pawn)
  (`KismetSystemLibrary.PrintString` "I SEE U"))

(event `self.ReceiveAnyDamage`
  (params (Damage :type "Float (single-precision)") (DamageType :type "DamageType Object Reference") (InstigatedBy :type "Controller Object Reference") (DamageCauser :type "Actor Object Reference"))
  ; taking damage
  (bind _output_get (set `self.health` (- (`self.health`) Damage)))
  (if (>= 0.0 _output_get)
    (`BlackboardComponent.SetValueAsBool` (`AIBlueprintHelperLibrary.GetBlackboard` (`AIBlueprintHelperLibrary.GetAIController` self)) "isDefeated" true)
    (`KismetSystemLibrary.PrintString` "ow")))

(fn `Ragdoll`
  (locals (NewLocalVar :type "Vector Structure" :default (0.0 0.0 0.0)))
  (bind _mesh (`self.Mesh`))
  (bind _pelvis (`self.pelvis`))
  ; Setup simulate physics
  (`PrimitiveComponent.SetCollisionProfileName` _mesh "Ragdoll" true)
  (`SkeletalMeshComponent.SetAllBodiesBelowSimulatePhysics` _mesh _pelvis true true)
  ; Keep ragdoll momentum
  (`SkeletalMeshComponent.AddImpulseToAllBodiesBelow` _mesh (`CharacterMovementComponent.GetLastUpdateRequestedVelocity` (`self.CharacterMovement`)) _pelvis false true))

(fn `UserConstructionScript`
  (set `self.health` 100.0))