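; GA_HipCheck is a Gameplay Ability for a melee hip-check attack that damages and knocks back pawns.
; It plays the montage, then waits once for the Notify.DoTrace event to sphere-trace at the avatar's pelvis socket, with debug drawing.
; Each hit receives set-by-caller damage, knockback and a brief invulnerability effect intended to prevent repeat hits.
; The ability ends in that event path, with no montage-interruption handling.
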(event `self.K2_ActivateAbility`
  (bind _returnvalue (`SceneComponent.GetSocketLocation` (`Actor.RootComponent` (`self.GetAvatarActorFromActorInfo`)) "pelvisSocket"))
  (if true
    ; Play HipCheck montage and wait for its notify DoTrace.
    (`|PlayMontage` (`self.GetOwningComponentFromActorInfo`) "/Game/GOBLINA/GoblinTest/Assets/AnimMontage/SK_HipCheck_Montage.SK_HipCheck_Montage"
      (:`then`
        (`AbilityTask_WaitGameplayEvent.WaitGameplayEvent` (struct :`TagName` "Notify.DoTrace") null true
          (:`EventReceived`
            ; Do a sphere trace around Pelvis socket
            (bind _outhits (`KismetSystemLibrary.SphereTraceMultiForObjects` :`Start` _returnvalue :`End` _returnvalue :`Radius` 100.0 :`ObjectTypes` (`|MakeArray` "ObjectTypeQuery3" :!type "EObjectTypeQuery Enum") :`DrawDebugType` "ForDuration" :`DrawTime` 1.5))
            (for _array_element _outhits
              (`|ExecutionSequence`
                (:`then_0`
                  ;[0.15 0 0 0.5] Apply Damage to target by tag Event.Damage
                  (bind _returnvalue_2 (`AbilitySystemBlueprintLibrary.AssignTagSetByCallerMagnitude` (`self.MakeOutgoingGameplayEffectSpec` "/Game/GOBLINA/GAS_TEST/Effects/GFX_TakeDamage.GFX_TakeDamage_C") (struct :`TagName` "Event.Damage") -100.0))
                  (bind _returnvalue_3 (`AbilitySystemBlueprintLibrary.AbilityTargetDataFromHitResult` _array_element))
                  (`self.K2_ApplyGameplayEffectSpecToTarget` _returnvalue_2 _returnvalue_3))
                (:`then_1`
                  ;[0.15 0.1415 0 0.5] Apply Knockback to target
                  (`self.BP_ApplyGameplayEffectToTarget` _returnvalue_3 "/Game/GOBLINA/GAS_TEST/Effects/GFX_Knockback.GFX_Knockback_C"))
                (:`then_2`
                  ;[0.02162 0 0.15 0.5] Apply Immunity - ensure target is only hit once by this attack
                  ; default is 0.5 s
                  (`self.BP_ApplyGameplayEffectToTarget` _returnvalue_3 "/Game/GOBLINA/GAS_TEST/Effects/GFX_Invulnerable.GFX_Invulnerable_C"))))
            (`self.K2_EndAbility`)))))))