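; GA_HipCheck is a Gameplay Ability for a hip check attack that damages nearby pawns.
; On activation it plays the hip check montage and waits once for the Notify.DoTrace gameplay event, timed to an anim notify.
; The event runs a debug-drawn sphere trace at the avatar's pelvis socket and applies GFX_ApplyDamage to each hit.
; The graph has no EndAbility call.
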(event `self.K2_ActivateAbility`
  (bind _returnvalue (`SceneComponent.GetSocketLocation` (`Actor.RootComponent` (`self.GetAvatarActorFromActorInfo`)) "pelvisSocket"))
  (if true
    (`|PlayMontage` (`self.GetOwningComponentFromActorInfo`) "/Game/GOBLINA/GoblinTest/Assets/AnimMontage/SK_HipCheck_Montage.SK_HipCheck_Montage"
      (:`then`
        (`AbilityTask_WaitGameplayEvent.WaitGameplayEvent` (struct :`TagName` "Notify.DoTrace") null true
          (:`EventReceived`
            ; Do a sphere trace when the AnimNotify triggers
            (bind _outhits (`KismetSystemLibrary.SphereTraceMultiForObjects` :`Start` _returnvalue :`End` _returnvalue :`Radius` 100.0 :`ObjectTypes` (`|MakeArray` "ObjectTypeQuery3" :!type "EObjectTypeQuery Enum") :`DrawDebugType` "ForDuration" :`DrawTime` 1.5))
            (for _array_element _outhits
              (`self.BP_ApplyGameplayEffectToTarget` (`AbilitySystemBlueprintLibrary.AbilityTargetDataFromHitResult` _array_element) "/Game/GOBLINA/GAS_TEST/GFX_ApplyDamage.GFX_ApplyDamage_C"))))))))